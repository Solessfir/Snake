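; BP_Wall is a Snake game boundary that wraps the snake around to the other side of the 10 m play zone.
; When its OverlapBox detects a BP_SnakeHead, it calls TeleportSnake with the box location, the reversed wall forward vector and a destination offset along the forward vector.
; The construction script turns off the box's collision when DisableOverlap is set.
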(event `self.OverlapBox.OnComponentBeginOverlap`
  (params (OverlappedComponent :type "PrimitiveComponent Object Reference") (OtherActor :type "Actor Object Reference") (OtherComp :type "PrimitiveComponent Object Reference") (OtherBodyIndex :type Integer) (bFromSweep :type Boolean) (SweepResult :type "HitResult Structure (by ref)"))
  (bind _returnvalue (`self.GetActorForwardVector`))
  (bind _asbp_snake_head (cast `/Game/Snake/Blueprints/BP_SnakeHead` OtherActor))
  (`/Game/Snake/Blueprints/BP_SnakeHead.Teleport Snake` _asbp_snake_head (`SceneComponent.K2_GetComponentLocation` (`self.OverlapBox`)) (* _returnvalue -1.0) (+ (`self.K2_GetActorLocation`) (* _returnvalue 1050.0))))

(fn `UserConstructionScript`
  (if (`self.bDisableOverlap`)
    (`PrimitiveComponent.SetCollisionEnabled` (`self.OverlapBox`) "NoCollision")))