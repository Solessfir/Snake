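; Game mode for a Snake game that manages the main menu, game start and timed item spawning.
; On begin play it shows the menu, precomputes a grid of spawn locations and binds to the Play button.
; Starting play switches to game-only input, broadcasts game start and runs a looping timer alongside a delayed first BP_Item spawn at a random grid point.
; ShowMenu stops the timer and passes game-over state and score to the menu.
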(event `self.ReceiveBeginPlay`
  (bind _returnvalue (`|CreateWidget` "/Game/Snake/Blueprints/Widgets/WBP_MainMenu.WBP_MainMenu_C" (`GameplayStatics.GetPlayerController` 0)))
  (bind _output_get (set `self.MainMenu` _returnvalue))
  (`UserWidget.AddToViewport` _output_get 0)
  (`self.Generate Item Spawn Locations`)
  (add `/Game/Snake/Blueprints/Widgets/WBP_MainMenu.OnPlayButtonPressed` (`self.MainMenu`) (`|CreateDelegate` :!event `Bind Spawn Item Event`)))

(event `Bind Spawn Item Event`
  (bind _returnvalue (`KismetSystemLibrary.K2_SetTimerDelegate` (`|CreateDelegate` :!event `Spawn Item in Random Location`) 5.0 true))
  (set `self.TimerHandle` _returnvalue)
  (`WidgetBlueprintLibrary.SetInputMode_GameOnly` (`GameplayStatics.GetPlayerController` 0))
  (`self.OnGameStarted`)
  (`KismetSystemLibrary.Delay` 1.0)
  (`self.Spawn Item in Random Location`))

(event `Generate Item Spawn Locations`
  (for _index (range -9 10)
    (for _index_2 (range -9 10)
      (`KismetArrayLibrary.Array_Add` (`self.SpawnLocations`) (`KismetMathLibrary.MakeVector` (* _index 50.0) (* _index_2 50.0) 57.2)))))

(event `Spawn Item in Random Location`
  (bind _spawnlocations (`self.SpawnLocations`))
  (`|SpawnActorFromClass` "/Game/Snake/Blueprints/BP_Item.BP_Item_C" (`KismetMathLibrary.MakeTransform` (`|GetArrayItem` _spawnlocations (`KismetMathLibrary.RandomInteger` (`KismetArrayLibrary.Array_LastIndex` _spawnlocations)))) "AlwaysSpawn" "OverrideRootScale" null null))

(event `Show Menu`
  (params (bGameOver :type Boolean) (Score :type Integer))
  (`KismetSystemLibrary.K2_ClearAndInvalidateTimerHandle` (`self.TimerHandle`))
  (`/Game/Snake/Blueprints/Widgets/WBP_MainMenu.Show Menu` (`self.MainMenu`) bGameOver Score))

(fn `UserConstructionScript`)