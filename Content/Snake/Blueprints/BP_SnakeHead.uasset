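; Player-controlled head of a Snake game that grows and speeds up on item pickups and ends the game on hitting its body.
; Tick moves it by direct location updates along an input-set direction that blocks reversals, easing head rotation.
; Each spawned body part follows the previous one, and teleports pass a waypoint to the first part behind a resettable DoOnce.
; GM_Snake handles start and menus, while flip-flopped tick pauses movement and WBP_HUD shows score and speed.
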(event `self.ReceiveBeginPlay`
  (bind _asgm_snake (cast `/Game/Snake/Blueprints/GM_Snake` (`GameplayStatics.GetGameMode`)))
  (bind _output_get (set `self.GameMode` _asgm_snake))
  (add `/Game/Snake/Blueprints/GM_Snake.OnGameStarted` _output_get (`|CreateDelegate` :!event `Custom Begin Play`)) ; Tell when Player press Play button
)

(event `Custom Begin Play`
  (bind _hud (`self.HUD`))
  (`/Engine/EditorBlueprintResources/StandardMacros.IsValid` _hud ; If HUD Valid - means player pressed Pause button
    (:`Is Valid`
      (`Widget.SetVisibility` _hud "Visible"))
    (:`Is Not Valid`
      (bind _returnvalue (`|CreateWidget` "/Game/Snake/Blueprints/Widgets/WBP_HUD.WBP_HUD_C" (`GameplayStatics.GetPlayerController` 0)))
      (bind _output_get (set `self.HUD` _returnvalue))
      (`/Game/Snake/Blueprints/Widgets/WBP_HUD.Update Text` _output_get (`KismetArrayLibrary.Array_Length` (`self.SnakeParts`)) (`self.Speed`))
      (`UserWidget.AddToViewport` _output_get 0)))
  (`self.Toggle Tick`) ; Pause moement while Player in Pause Menu
)

(event `Toggle Tick`
  (bind _isa (`/Engine/EditorBlueprintResources/StandardMacros.FlipFlop`)
    (:`A`
      _)
    (:`B`
      _))
  (`self.SetActorTickEnabled` _isa))

(event `self.ReceiveTick`
  (params (DeltaSeconds :type "Float (single-precision)"))
  (`self.K2_SetActorLocation` (`self.GetSnakeVelocity`) false true) ; Don't want to use Floating Pawn Movement
  (`SceneComponent.K2_SetRelativeRotation` (`self.SnakeHead`) (`KismetMathLibrary.RInterpTo` (`SceneComponent.RelativeRotation` (`self.SnakeHead`)) (`KismetMathLibrary.Conv_VectorToRotator` (`self.MovementDirection`)) (`GameplayStatics.GetWorldDeltaSeconds`) 10.0) false false) ; Snake Head Rotation
)

(event `self.SphereCollision.OnComponentBeginOverlap`
  (params (OverlappedComponent :type "PrimitiveComponent Object Reference") (OtherActor :type "Actor Object Reference") (OtherComp :type "PrimitiveComponent Object Reference") (OtherBodyIndex :type Integer) (bFromSweep :type Boolean) (SweepResult :type "HitResult Structure (by ref)"))
  (bind _hud (`self.HUD`))
  (cast `/Game/Snake/Blueprints/BP_Item` OtherActor ; Is is Pickup Item?
    (:`then`
      (`self.AddSnakePart`)
      (`self.IncreaseSpeed`) ; Want to move faster
      (`/Engine/EditorBlueprintResources/StandardMacros.IsValid` _hud
        (:`Is Valid`
          (`/Game/Snake/Blueprints/Widgets/WBP_HUD.Update Text` _hud (* (`KismetArrayLibrary.Array_Length` (`self.SnakeParts`)) 10) (`self.Speed`)) ; Snake Body Parts * 10 = Score
        )))
    (:`CastFailed`
      (cast `/Game/Snake/Blueprints/BP_Wall` OtherActor ; Ok, is it Teleporter?
        (:`CastFailed`
          (`/Engine/EditorBlueprintResources/StandardMacros.DoOnce` false ; Then it's Snake Body = Game End
            (:`Completed`
              (`self.Toggle Tick`)
              (`Widget.RemoveFromParent` (`self.HUD`))
              (`/Game/Snake/Blueprints/GM_Snake.Show Menu` (`self.GameMode`) true (* (`KismetArrayLibrary.Array_Length` (`self.SnakeParts`)) 10)))))))))

(event `InputAction|Menu`
  (params (Key :type "Key Structure"))
  (:`Pressed`
    (`Widget.SetVisibility` (`self.HUD`) "Hidden")
    (`self.Toggle Tick`)
    (`/Game/Snake/Blueprints/GM_Snake.Show Menu` (`self.GameMode`) false 0) ; Game is NOT over, just Pause
  ))

(event `Teleport Snake`
  (params (InitialLocation :type "Vector Structure") (ForwardVector :type "Vector Structure") (NewLocation :type "Vector Structure"))
  (bind _output (`|GetArrayItem` (`self.SnakeParts`)))
  ;[1 1 1] Handle Snake body parts teleportation
  (`/Engine/EditorBlueprintResources/StandardMacros.DoOnce` false :!label _label ; Make sure Teleportation will work only once
    (:`Completed`
      (`/Engine/EditorBlueprintResources/StandardMacros.IsValid` _output ; It Player didn't pickup an Item and Teleported
        (:`Is Valid`
          (`/Game/Snake/Blueprints/BP_SnakeBody.Add New Target Location` _output InitialLocation ForwardVector))
        (:`Is Not Valid`
          _))
      (`self.K2_TeleportTo` NewLocation)
      (`KismetSystemLibrary.Delay` 0.2)
      (`self.Reset DoOnce Teleport`))))

(event `Reset DoOnce Teleport`
  ;[1 1 1] Handle Snake body parts teleportation
  (goto _label :!via `Reset`))

(event `InputAction|MoveUp`
  (params (Key :type "Key Structure"))
  ;[1 1 1] Movement
  (:`Pressed`
    (if (!= (`self.MovementDirection`) (-1.0 0.0 0.0) :`ErrorTolerance` 0.0)
      (set `self.MovementDirection` (1.0 0.0 0.0)))))

(event `InputAction|MoveDown`
  (params (Key :type "Key Structure"))
  ;[1 1 1] Movement
  (:`Pressed`
    (if (!= (`self.MovementDirection`) (1.0 0.0 0.0) :`ErrorTolerance` 0.0)
      (set `self.MovementDirection` (-1.0 0.0 0.0)))))

(event `InputAction|MoveRight`
  (params (Key :type "Key Structure"))
  ;[1 1 1] Movement
  (:`Pressed`
    (if (!= (`self.MovementDirection`) (0.0 -1.0 0.0) :`ErrorTolerance` 0.0)
      (set `self.MovementDirection` (0.0 1.0 0.0)))))

(event `InputAction|MoveLeft`
  (params (Key :type "Key Structure"))
  ;[1 1 1] Movement
  (:`Pressed`
    (if (!= (`self.MovementDirection`) (0.0 1.0 0.0) :`ErrorTolerance` 0.0)
      (set `self.MovementDirection` (0.0 -1.0 0.0)))))

(fn `AddSnakePart`
  (bind (_returnvalue_location _returnvalue_rotation _returnvalue_scale) (`KismetMathLibrary.BreakTransform` (`self.GetTransform`)))
  (bind _snakeparts (`self.SnakeParts`))
  (bind _output (`|GetArrayItem` _snakeparts (`KismetArrayLibrary.Array_LastIndex` _snakeparts)))
  (bind (_returnvalue_location_2 _returnvalue_rotation_2 _returnvalue_scale_2) (`KismetMathLibrary.BreakTransform` (`self.GetTransform` _output)))
  (if (> (`KismetArrayLibrary.Array_Length` (`self.SnakeParts`)) 0)
    (bind _returnvalue (`|SpawnActorFromClass` "/Game/Snake/Blueprints/BP_SnakeBody.BP_SnakeBody_C" (`KismetMathLibrary.MakeTransform` (+ _returnvalue_location_2 (* (* (`self.GetActorForwardVector` _output) -1.0) 60.0)) _returnvalue_rotation_2 _returnvalue_scale_2) "AlwaysSpawn" "OverrideRootScale" self _output null))
    (`KismetArrayLibrary.Array_Add` (`self.SnakeParts`) _returnvalue)
    (else
      (bind _returnvalue_2 (`|SpawnActorFromClass` "/Game/Snake/Blueprints/BP_SnakeBody.BP_SnakeBody_C" (`KismetMathLibrary.MakeTransform` (+ _returnvalue_location (* (* (`SceneComponent.GetForwardVector` (`self.SnakeHead`)) -1.0) 60.0)) _returnvalue_rotation _returnvalue_scale) "AlwaysSpawn" "OverrideRootScale" self self null))
      (`KismetArrayLibrary.Array_Add` (`self.SnakeParts`) _returnvalue_2))))

(fn `GetSnakeVelocity`
  (returns (ReturnValue :type "Vector Structure"))
  (return (+ (`self.K2_GetActorLocation`) (* (`self.MovementDirection`) (* (`GameplayStatics.GetWorldDeltaSeconds`) (`self.Speed`))))))

(fn `IncreaseSpeed`
  (set `self.Speed` (+ (`self.Speed`) 10.0)))

(fn `UserConstructionScript`)