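; Snake body segment that trails its parent part at a set spacing, interpolating with the head's speed.
; For wall teleports, it moves through queued target locations, easing speed by the head's direction against the stored forward vector.
; On reaching a target, it broadcasts OnLocationReached for child segments, then jumps to the next target or near its parent.
; It enables query collision after a delay and destroys itself without a valid parent.
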(event `self.ReceiveBeginPlay`
  (bind _parentsnakepart (`self.ParentSnakePart`)
    (:`then`
      (`|ExecutionSequence`
        (:`then_0`
          (bind _asbp_snake_body (cast `/Game/Snake/Blueprints/BP_SnakeBody` _parentsnakepart)) ; We need to bind only Snake Body parts
          (add `self.OnLocationReached` _asbp_snake_body (`|CreateDelegate` :!event `Add New Target Location`)) ; This will handle Teleportation
        )
        (:`then_1`
          (`self.SetActorTickEnabled` true) ; Good to go!
          (`KismetSystemLibrary.Delay` 1.0)
          (`PrimitiveComponent.SetCollisionEnabled` (`self.StaticMesh`) "QueryOnly"))))
    (:`else`
      (`self.K2_DestroyActor`) ; In case something brakes
    )))

(event `self.ReceiveTick`
  (params (DeltaSeconds :type "Float (single-precision)"))
  (bind _returnvalue (`self.K2_GetActorLocation` (`self.ParentSnakePart`)))
  (bind _asbp_snake_head (cast `/Game/Snake/Blueprints/BP_SnakeHead` (`self.GetOwner`) :!pure true))
  (bind _returnvalue_2 (`KismetMathLibrary.FindLookAtRotation` (`self.K2_GetActorLocation`) _returnvalue))
  (bind _returnvalue_3 (`KismetMathLibrary.VSize` (`/Game/Snake/Blueprints/BP_SnakeHead.GetSnakeVelocity` _asbp_snake_head)))
  (`SceneComponent.K2_SetRelativeRotation` (`self.StaticMesh`) _returnvalue_2 false false) ; Update mesh rotation, so we can get correct forward vector
  (if (> (`KismetArrayLibrary.Array_Length` (`self.TargetLocations`)) 0)
    (`self.K2_SetActorLocation` (`KismetMathLibrary.VInterpTo_Constant` (`self.K2_GetActorLocation`) (`|GetArrayItem` (`self.TargetLocations`)) (`GameplayStatics.GetWorldDeltaSeconds`) (`|EaseFunction` "EaseInOut" (`self.NormalizedDotProduct` (`self.TargetForwardVector`) (`/Game/Snake/Blueprints/BP_SnakeHead.MovementDirection` _asbp_snake_head)) (/ _returnvalue_3 2.0) _returnvalue_3 0.1)) false true) ; Follow teleport location, NOT Parent
    (if (== (`self.K2_GetActorLocation`) (`|GetArrayItem` (`self.TargetLocations`)) :`ErrorTolerance` 1.0)
      (`self.OnLocationReached` (`|GetArrayItem` (`self.TargetLocations`)) (`self.TargetForwardVector`)) ; Tell the child to set new Target Location
      (`KismetArrayLibrary.Array_Remove` (`self.TargetLocations`)) ; Snake part already reached this location, so we don't need it anymore
      (`self.Reset Position`))
    (else
      (`self.K2_SetActorLocation` (`KismetMathLibrary.VInterpTo` (`self.K2_GetActorLocation`) (+ (* (* (`KismetMathLibrary.GetForwardVector` _returnvalue_2) -1.0) (`self.DistanceBetweenParts`)) _returnvalue) (`GameplayStatics.GetWorldDeltaSeconds`) (/ (`KismetMathLibrary.VSize` (`/Game/Snake/Blueprints/BP_SnakeHead.GetSnakeVelocity` (cast `/Game/Snake/Blueprints/BP_SnakeHead` (`self.GetOwner`) :!pure true))) 10.0)) false true))))

(event `Reset Position`
  (bind _parentsnakepart (`self.ParentSnakePart`)
    (:`then`
      (bind _returnvalue (`self.K2_GetActorLocation` _parentsnakepart))
      (`self.K2_SetActorLocation` (select `bool` (> (`KismetArrayLibrary.Array_Length` (`self.TargetLocations`)) 0) :`false` (+ (* (`KismetMathLibrary.GetForwardVector` (`KismetMathLibrary.FindLookAtRotation` (`self.K2_GetActorLocation`) _returnvalue)) (`self.DistanceBetweenParts`)) _returnvalue) :`true` (`|GetArrayItem` (`self.TargetLocations`))) false true))
    (:`else`)))

(event `Add New Target Location` :!signature `self.OnLocationReached`
  (params (Location :type "Vector Structure") (ForwardVector :type "Vector Structure"))
  (`KismetArrayLibrary.Array_Add` (`self.TargetLocations`) Location)
  (set `self.TargetForwardVector` ForwardVector) ; Need to control Snake tail teleportation interpolation speed
)

(fn `UserConstructionScript`)